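; Quest giver NPC that shows a camera-facing interact prompt while the player character is in its trigger radius.
; Repeated Interact calls step through the Dialogue array, then open a quest widget filled from Quests; a further call closes it.
; Leaving the radius resets dialogue and tears down the UI.
; A self-repeating AI roam uses WalkRadius, zeroed during dialogue, but nothing here starts it.
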(event OnComponentBeginOverlap(TriggerRadius)
  (params (OverlappedComponent :type Primitive%20Component%20Object%20Reference) (OtherActor :type Actor%20Object%20Reference) (OtherComp :type Primitive%20Component%20Object%20Reference) (OtherBodyIndex :type Integer) (bFromSweep :type Boolean) (SweepResult :type Hit%20Result%20Structure%20%28by%20ref%29))
  (Utilities|Casting|CastToThirdPersonCharacter OtherActor)
  (Rendering|SetVisibility (Variables|Default|GetInteract%20Widget) true false))

(event OnComponentEndOverlap(TriggerRadius)
  (params (OverlappedComponent :type Primitive%20Component%20Object%20Reference) (OtherActor :type Actor%20Object%20Reference) (OtherComp :type Primitive%20Component%20Object%20Reference) (OtherBodyIndex :type Integer))
  (bind _returnvalue (Game|GetPlayerController 0))
  (Utilities|Casting|CastToThirdPersonCharacter OtherActor)
  (Rendering|SetVisibility (Variables|Default|GetInteract%20Widget) false false)
  (Utilities|FlowControl|Sequence
    (:then_0
      (Widget|RemovefromParent (Variables|Default|GetDialogue%20Widget))
      (Variables|Default|SetDialogue%20Widget 0)
      (Variables|Default|SetDialogueIndex 0)
      (Variables|Default|SetDialogueOpened? false)
      (CallFunction|OpenQuestsWidget))
    (:then_1
      (Widget|RemovefromParent (Variables|Default|GetQuest%20Widget))
      (Variables|/Script/Engine.PlayerController|SetbShowMouseCursor _returnvalue false)
      (Input|SetInputModeGameOnly _returnvalue)
      (Variables|Default|SetWidget%20Active false)
      (Variables|Default|Setwalk%20radius 1e+03))))

(event Custom|Roaming
  (AI|AIMoveTo self (.RandomLocation (AI|Navigation|GetRandomReachablePointinRadius (Transformation|GetWorldLocation (Variables|Character|GetMesh)) (Variables|Default|Getwalk%20radius) 0 0)) 0 5.0 false
    (:OnSuccess
      (Utilities|FlowControl|Delay (Math|Random|RandomFloatinRange 1.0 3.0))
      (CallFunction|Roaming))))

(event Custom|Close%20Widget
  (bind _returnvalue (Game|GetPlayerController 0))
  (Widget|RemovefromParent (Variables|Default|GetQuest%20Widget))
  (Variables|/Script/Engine.PlayerController|SetbShowMouseCursor _returnvalue false)
  (Input|SetInputModeGameOnly _returnvalue)
  (Variables|Default|SetWidget%20Active false)
  (Variables|Default|Setwalk%20radius 1e+03))

(event Custom|Open%20Quests%20Widget
  (bind _returnvalue (UserInterface|CreateWidget "/Game/QuestSystem-Sample/WB_QuestGiverWB.WB_QuestGiverWB_C"))
  (bind _output_get (Variables|Default|SetQuest%20Widget _returnvalue))
  (UserInterface|Viewport|AddtoViewport _output_get 0)
  (Variables|Default|SetWidget%20Active true)
  (Variables|/Game/QuestSystem-Sample/WB_QuestGiverWB.WB_QuestGiverWB_C|SetQuest%20Giver%20BP (Variables|Default|GetQuest%20Widget) self)
  (for _array_element (Variables|Default|GetQuests)
    (Default|AddQuest (Variables|Default|GetQuest%20Widget) _array_element)))

(event EventTick
  (params (DeltaSeconds :type Float%20%28single-precision%29))
  (Transformation|SetWorldRotation (Variables|Default|GetInteract%20Widget) (Math|Rotator|FindLookatRotation (Transformation|GetWorldLocation (Variables|Default|GetInteract%20Widget)) (Transformation|GetWorldLocation (Variables|/Script/Engine.Actor|GetRootComponent (Game|GetPlayerCameraManager 0)))) false false))

(event EventInteract
  (bind _returnvalue (Game|GetPlayerController 0))
  (bind _returnvalue_2 (Game|GetPlayerController 0))
  (if (not (Variables|Default|GetWidget%20Active))
    (if (not (Variables|Default|GetDialogueOpened?))
      (Variables|Default|Setwalk%20radius 0.0)
      (bind _returnvalue_3 (UserInterface|CreateWidget "/Game/QuestSystem-Sample/WB_QuestGIverDialogue.WB_QuestGIverDialogue_C"))
      (bind _output_get (Variables|Default|SetDialogue%20Widget _returnvalue_3))
      (UserInterface|Viewport|AddtoViewport _output_get 0)
      (Variables|Default|SetDialogueOpened? true)
      (Rendering|Components|TextRender|SetText (Variables|/Game/QuestSystem-Sample/WB_QuestGIverDialogue.WB_QuestGIverDialogue_C|GetDialogueText (Variables|Default|GetDialogue%20Widget)) (Utilities|Text|ToText(String) (Utilities|Array|Get(acopy) (Variables|Default|GetDialogue) (Variables|Default|GetDialogueIndex))))
      (Math|Integer|IncrementInt (Variables|Default|GetDialogueIndex)
        (:%20%20
          (Variables|/Script/Engine.PlayerController|SetbShowMouseCursor _returnvalue_2 true)
          (Input|SetInputModeGameandUI _returnvalue_2 (Variables|Default|GetQuest%20Widget) "DoNotLock" true)))
      (else
        (Rendering|Components|TextRender|SetText (Variables|/Game/QuestSystem-Sample/WB_QuestGIverDialogue.WB_QuestGIverDialogue_C|GetDialogueText (Variables|Default|GetDialogue%20Widget)) (Utilities|Text|ToText(String) (Utilities|Array|Get(acopy) (Variables|Default|GetDialogue) (Variables|Default|GetDialogueIndex))))
        (Math|Integer|IncrementInt (Variables|Default|GetDialogueIndex)
          (:%20%20
            (if (> (Variables|Default|GetDialogueIndex) (Utilities|Array|Length (Variables|Default|GetDialogue)))
              (Widget|RemovefromParent (Variables|Default|GetDialogue%20Widget))
              (Variables|Default|SetDialogue%20Widget 0)
              (Variables|Default|SetDialogueIndex 0)
              (Variables|Default|SetDialogueOpened? false)
              (CallFunction|OpenQuestsWidget))))))
    (else
      (Variables|Default|Setwalk%20radius 1e+03)
      (Widget|RemovefromParent (Variables|Default|GetQuest%20Widget))
      (Variables|/Script/Engine.PlayerController|SetbShowMouseCursor _returnvalue false)
      (Input|SetInputModeGameOnly _returnvalue)
      (Variables|Default|SetWidget%20Active false)
      (Variables|Default|Setwalk%20radius 1e+03))))

(event EventBeginPlay)

(fn ConstructionScript)