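; Quest component that tracks the active quest's objectives and drives the player's quest HUD, which it creates hidden on BeginPlay.
; Events push the quest name and objectives to the widget.
; TalktoNPC marks objectives matching the given NPC complete, updates the HUD and increments a counter.
; The completion check tests objective count >= counter, so the quest-completed animation can play from the first completed objective rather than only the last.
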(event Custom|Set%20Active%20Quest%20Text
  (bind _quest_hud_widget (Variables|Default|GetQuest%20Hud%20Widget))
  (bind _activequesttext (Variables|/Game/QuestSystem-Sample/WB_QuestPlayerHud.WB_QuestPlayerHud_C|GetActiveQuestText _quest_hud_widget))
  (Rendering|Components|TextRender|SetText _activequesttext (Utilities|Text|ToText(String) (.Name (Utilities|Struct|BreakS_Quest (Variables|Default|GetActive%20Quest)))))
  (Widget|SetVisibility _activequesttext "Visible")
  (Default|ShowQuestPanel (Variables|Default|GetQuest%20Hud%20Widget)))

(event Custom|Set%20Objectives%20Text
  (Default|FillObjectives (Variables|Default|GetQuest%20Hud%20Widget) (.objectives (Variables|Default|GetActive%20Quest))))

(event Custom|Talk%20to%20NPC
  (params (NPC :type Actor%20Object%20Reference))
  (for _array_element (.objectives (Variables|Default|GetActive%20Quest))
    (if (and (.IsTalkNPCObjective (Utilities|Struct|BreakS_QuestObjective _array_element)) (== NPC (.TalktoNPC (Utilities|Struct|BreakS_QuestObjective _array_element))))
      (|SetBy-RefVar _array_element (Utilities|Struct|MakeS_QuestObjective (.NameAim (Utilities|Struct|BreakS_QuestObjective _array_element)) true (.TalktoNPC (Utilities|Struct|BreakS_QuestObjective _array_element)) (.IsTalkNPCObjective (Utilities|Struct|BreakS_QuestObjective _array_element))))
      (Default|CompleteObjective (Variables|Default|GetQuest%20Hud%20Widget) _array_element)
      (CallFunction|ObjectiveCompleted)
      (Development|PrintString "Complete Objecteive"))))

(event Custom|Objective%20Completed
  (Math|Integer|IncrementInt (Variables|Default|GetQuest%20Objective%20Completed)
    (:%20%20
      (if (>= (Utilities|Array|Length (.objectives (Variables|Default|GetActive%20Quest))) (Variables|Default|GetQuest%20Objective%20Completed))
        (Development|PrintString "QUEST COMPLETED")
        (Default|PlayQuestCompletedAnimation (Variables|Default|GetQuest%20Hud%20Widget))))))

(event EventBeginPlay
  (bind _returnvalue (UserInterface|CreateWidget "/Game/QuestSystem-Sample/WB_QuestPlayerHud.WB_QuestPlayerHud_C"))
  (bind _output_get (Variables|Default|SetQuest%20Hud%20Widget _returnvalue))
  (UserInterface|Viewport|AddtoViewport _output_get 0)
  (Default|HideQuestPanel (Variables|Default|GetQuest%20Hud%20Widget)))